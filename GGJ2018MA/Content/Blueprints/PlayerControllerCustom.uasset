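; Custom player controller that turns gamepad and keyboard input into direction rotation on its possessed Player pawn.
; Left-stick X and Y axes are scaled by AxisMultiplier and both feed yaw into AddDirectionRotation, with Y inverted.
; On Tick, the controller with PlayerIndex 1 polls J and L on player controller 0 to yaw left or right, letting a second player share that keyboard.
; PlayerIndex is exposed through simple get and set functions.
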(event `InputAxisKey|Gamepad_LeftX`
  (params (AxisValue :type "Float (single-precision)"))
  (bind _asplayer (cast `/Game/Blueprints/Player` (`self.K2_GetPawn` self))
    (:`then`
      (`/Game/Blueprints/Player.AddDirectionRotation` _asplayer (`KismetMathLibrary.MakeRotator` 0.0 0.0 (+ 0.0 (`KismetMathLibrary.BreakVector2D` (* (`KismetMathLibrary.MakeVector2D` AxisValue) (`self.AxisMultiplier`)))))))
    (:`CastFailed`
      (`KismetSystemLibrary.PrintString` "Player cast failed" false false (struct :`R` 0.666667 :`A` 1.0) 10.0))))

(event `InputAxisKey|Gamepad_LeftY`
  (params (AxisValue :type "Float (single-precision)"))
  (bind _asplayer (cast `/Game/Blueprints/Player` (`self.K2_GetPawn` self))
    (:`then`
      (`/Game/Blueprints/Player.AddDirectionRotation` _asplayer (`KismetMathLibrary.MakeRotator` 0.0 0.0 (* (`.Y` (`KismetMathLibrary.BreakVector2D` (* (`KismetMathLibrary.MakeVector2D` 0.0 AxisValue) (`self.AxisMultiplier`)))) -1.0))))
    (:`CastFailed`
      (`KismetSystemLibrary.PrintString` "Player cast failed" false false (struct :`R` 0.666667 :`A` 1.0) 10.0))))

(event `self.ReceiveTick`
  (params (DeltaSeconds :type "Float (single-precision)"))
  (if (== (`self.playerIndex`) 1)
    (`|ExecutionSequence`
      (:`then_0`
        (if (`self.IsInputKeyDown` (`GameplayStatics.GetPlayerController` 0) "J")
          (bind _asplayer (cast `/Game/Blueprints/Player` (`self.K2_GetPawn`))
            (:`then`
              (`/Game/Blueprints/Player.AddDirectionRotation` _asplayer (`KismetMathLibrary.MakeRotator` 0.0 0.0 -1.0)))
            (:`CastFailed`
              (`KismetSystemLibrary.PrintString` "Player cast failed" false false (struct :`R` 0.666667 :`A` 1.0) 10.0)))))
      (:`then_1`
        (if (`self.IsInputKeyDown` (`GameplayStatics.GetPlayerController` 0) "L")
          (bind _asplayer_2 (cast `/Game/Blueprints/Player` (`self.K2_GetPawn`))
            (:`then`
              (`/Game/Blueprints/Player.AddDirectionRotation` _asplayer_2 (`KismetMathLibrary.MakeRotator` 0.0 0.0 1.0)))
            (:`CastFailed`
              (`KismetSystemLibrary.PrintString` "Player cast failed" false false (struct :`R` 0.666667 :`A` 1.0) 10.0))))))))

(fn `GetPlayerIndex`
  (returns (index :type Integer))
  (return (`self.playerIndex`)))

(fn `SetPlayerIndex`
  (params (index :type Integer))
  (set `self.playerIndex` index))

(fn `UserConstructionScript`)