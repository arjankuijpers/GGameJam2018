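; FinishPoint is a goal actor that ends the round when a player reaches it.
; On BeginPlay it finds and stores the level's GameController, printing an error if none exists.
; When a Player enters its sphere collider, it gets that player's index, prints a win message and passes the index to GameController's FinishRound.
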(event `self.ReceiveBeginPlay`
  (bind _outactors (`GameplayStatics.GetAllActorsOfClass` "/Game/Blueprints/GameController.GameController_C"))
  (bind _output (`|GetArrayItem` _outactors))
  (`/Engine/EditorBlueprintResources/StandardMacros.IsValid` _output
    (:`Is Valid`
      (set `self.gameControllerRef` _output))
    (:`Is Not Valid`
      (`KismetSystemLibrary.PrintString` "GameController not found!" true true (struct :`R` 1.0 :`B` 0.035882 :`A` 1.0) 20.0))))

(event `self.SphereCollider.OnComponentBeginOverlap`
  (params (OverlappedComponent :type "PrimitiveComponent Object Reference") (OtherActor :type "Actor Object Reference") (OtherComp :type "PrimitiveComponent Object Reference") (OtherBodyIndex :type Integer) (bFromSweep :type Boolean) (SweepResult :type "HitResult Structure (by ref)"))
  (`KismetSystemLibrary.PrintString` "FinishPoint OnBeginOverlap" true true (struct :`R` 0.703998 :`G` 1.0 :`B` 0.507654 :`A` 1.0) 5.0)
  (if (`KismetMathLibrary.ClassIsChildOf` (`GameplayStatics.GetObjectClass` OtherActor) "/Game/Blueprints/Player.Player_C")
    (bind _asplayer (cast `/Game/Blueprints/Player` OtherActor))
    (bind _getplayerindex (`/Game/Blueprints/Player.GetPlayerIndex` _asplayer))
    (`KismetSystemLibrary.PrintString` (`KismetStringLibrary.Concat_StrStr` "Win, Player: " (`KismetStringLibrary.Conv_IntToString` _getplayerindex)) true true (struct :`R` 0.538257 :`G` 0.420212 :`B` 1.0 :`A` 1.0) 10.0)
    (`/Game/Blueprints/GameController.FinishRound` (`self.gameControllerRef`) _getplayerindex)))

(fn `UserConstructionScript`)