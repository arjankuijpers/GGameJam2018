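; Obstacle actor that exposes a speed multiplier and changes its material color to show whether players are active in it.
; On BeginPlay it creates a dynamic material from the static mesh's first material.
; Two color functions keep a count of active players and set the passthrough color parameter, restoring the inactive color only when the count reaches zero.
; The overlap events are empty, with their player checks disconnected, so nothing here calls those functions.
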(event `self.ReceiveBeginPlay`
  (bind _staticmesh (`self.StaticMesh`))
  (bind _returnvalue (`PrimitiveComponent.CreateDynamicMaterialInstance` _staticmesh 0 (`|GetArrayItem` (`MeshComponent.GetMaterials` _staticmesh))))
  (set `self.dynamicMaterial` _returnvalue))

(event `self.ReceiveActorBeginOverlap`
  (params (OtherActor :type "Actor Object Reference")))

(event `self.ReceiveActorEndOverlap`
  (params (OtherActor :type "Actor Object Reference")))

(fn `GetSpeedMultiplier`
  (returns (speedMultiplier :type "Float (double-precision)"))
  (return (`self.speedMultiplier`)))

(fn `SetColorNoPlayerActive`
  (`/Engine/EditorBlueprintResources/StandardMacros.IsValid` (`self.dynamicMaterial`)
    (:`Is Valid`
      (`/Engine/EditorBlueprintResources/StandardMacros.DecrementInt` (`self.playersActive`)
        (:`  `
          (if (== (`self.playersActive`) 0)
            (`MaterialInstanceDynamic.SetVectorParameterValue` (`self.dynamicMaterial`) "ColorPlayerPassthrough" (`self.ColorNoPlayerActive`))
            (`KismetSystemLibrary.PrintString` (`KismetStringLibrary.Concat_StrStr` "Obstacle Player no longer Active: " (`KismetStringLibrary.Conv_IntToString` (`self.playersActive`))) false false (struct :`G` 0.66 :`B` 1.0 :`A` 1.0) 5.0)))))))

(fn `SetColorPlayerActive`
  (`/Engine/EditorBlueprintResources/StandardMacros.IsValid` (`self.dynamicMaterial`)
    (:`Is Valid`
      (`/Engine/EditorBlueprintResources/StandardMacros.IncrementInt` (`self.playersActive`)
        (:`  `
          (`MaterialInstanceDynamic.SetVectorParameterValue` (`self.dynamicMaterial`) "ColorPlayerPassthrough" (`self.ColorPlayerActive`))
          (`KismetSystemLibrary.PrintString` (`KismetStringLibrary.Concat_StrStr` "Obstacle Player Active: " (`KismetStringLibrary.Conv_IntToString` (`self.playersActive`))) false false (struct :`G` 0.66 :`B` 1.0 :`A` 1.0) 5.0))))))

(fn `UserConstructionScript`)