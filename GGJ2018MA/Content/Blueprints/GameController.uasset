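; Match controller actor that runs a multiplayer round from setup through countdown to the win screen.
; MakeGameReady reads the player count from GameInstanceMA, creates spawners at random positions within bounds, spawns players through them and builds the UI.
; GamePlayStart runs a looping-timer countdown, then activates player movement and switches the first controller's view to CameraActor.
; FinishRound stops movement, shows the winner and notifies the game instance.
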(fn `ActivatePlayerMovement`
  (`KismetSystemLibrary.PrintString` "Activate players" true true (struct :`R` 0.179174 :`G` 1.0 :`A` 1.0) 5.0)
  (for _array_element (`self.Spawners`)
    (bind _playerref (`/Game/Blueprints/Spawner.GetPlayerRef` _array_element))
    (`/Game/Blueprints/Player.SetMovementData` _playerref (`self.PlayerStartRotation`) (`self.playerSpeed`) (`self.playerRotationSpeed`))
    (`/Game/Blueprints/Player.ActivateMovement` _playerref)))

(fn `CountDownForStart`
  (`KismetSystemLibrary.PrintString` "Start Countdown" true true (struct :`R` 0.310078 :`B` 1.0 :`A` 1.0) 5.0)
  (bind _returnvalue (`KismetSystemLibrary.K2_SetTimer` self "CountDownUpdate" 1.0 true))
  (set `self.TimerHandle` _returnvalue)
  (`Widget.SetVisibility` (`self.CountDownUI`) "Visible")
  (`self.UpdateCountDownUI` (`self.CountDownTime`)))

(fn `CountDownUpdate`
  (`KismetSystemLibrary.PrintString` "Timer Update" true true (struct :`R` 0.7395 :`G` 1.0 :`A` 1.0))
  (`KismetSystemLibrary.PrintString` (`KismetStringLibrary.Concat_StrStr` "CD: " (`KismetStringLibrary.Conv_IntToString` (`self.CountDownTime`))) true true (struct :`R` 1.0 :`G` 0.770984 :`A` 1.0) 5.0)
  (`self.UpdateCountDownUI` (- (`self.CountDownTime`) 1))
  (bind _output_get (set `self.CountDownTime` (- (`self.CountDownTime`) 1)))
  (if (== _output_get 0)
    (`KismetSystemLibrary.K2_ClearAndInvalidateTimerHandle` (`self.TimerHandle`))
    (`KismetSystemLibrary.PrintString` "Clear CountDown Timer" true true (struct :`G` 1.0 :`B` 0.125167 :`A` 1.0) 5.0)
    (`self.ActivatePlayerMovement`)
    (`PlayerController.SetViewTargetWithBlend` (`GameplayStatics.GetPlayerController` 0) (`self.CameraActor`) 0.0 "VTBlend_Linear" 0.0 false)))

(fn `CreateAllSpawners`
  (`KismetSystemLibrary.PrintString` "Create All Spawners" true true (struct :`G` 0.66 :`B` 1.0 :`A` 1.0) 5.0)
  (for _ (range (`self.numPlayers`))
    ;[1 1 1] Creates spawner
    (bind _spawner (`self.CreateSpawnerRandomPosition`))
    (bind _returnvalue (`KismetArrayLibrary.Array_Add` (`self.Spawners`) _spawner))
    (`KismetSystemLibrary.PrintString` (`KismetStringLibrary.Concat_StrStr` "Create Spawner: " (`KismetStringLibrary.Conv_IntToString` _returnvalue)) true true (struct :`G` 0.66 :`B` 1.0 :`A` 1.0) 5.0))
  (`KismetSystemLibrary.PrintString` "Create All Spawners Done" true true (struct :`G` 0.340343 :`B` 1.0 :`A` 1.0) 5.0))

(fn `CreateSpawnerRandomPosition`
  (returns (Spawner :type "/Game/Blueprints/Spawner Object Reference"))
  (bind _position (`self.GetRandomPosVector`))
  (bind _returnvalue (`|SpawnActorFromClass` "/Game/Blueprints/Spawner.Spawner_C" (`KismetMathLibrary.Conv_VectorToTransform` _position) "AlwaysSpawn" "OverrideRootScale" self null))
  (return _returnvalue))

(fn `DeactivatePlayerMovement`
  (`KismetSystemLibrary.PrintString` "Deactivate players" true true (struct :`R` 0.179174 :`G` 1.0 :`A` 1.0) 5.0)
  (for _array_element (`self.Spawners`)
    (bind _playerref (`/Game/Blueprints/Spawner.GetPlayerRef` _array_element))
    (`/Game/Blueprints/Player.DeactivateMovement` _playerref)))

(fn `FinishRound`
  (params (playerIndexWin :type Integer))
  (if (< playerIndexWin (`self.numPlayers`))
    (`KismetSystemLibrary.PrintString` (`KismetTextLibrary.Conv_TextToString` (`|FormatText` "GameController: Player {0} Wins" playerIndexWin)))
    (`self.DeactivatePlayerMovement`)
    (`self.ShowWinLoseUI` (`|GetArrayItem` (`self.playerNames`) playerIndexWin) 1)
    (`/Game/Blueprints/GameInstanceMA.RoundCompleted` (`self.gameInstanceMA`) 0)
    (else
      (`KismetSystemLibrary.PrintString` "GameController::WinPlayerIndex out of bounds." true true (struct :`R` 1.0 :`B` 0.051847 :`A` 1.0) 20.0))))

(fn `GamePlayStart`
  (`KismetSystemLibrary.PrintString` "Game Play Start" true true (struct :`G` 0.300881 :`B` 1.0 :`A` 1.0) 5.0)
  (`self.CountDownForStart`))

(fn `GetRandomPosVector`
  (returns (position :type "Vector Structure"))
  (bind (_x _y) (`KismetMathLibrary.BreakVector2D` (`self.minRandomSpawnPosition`)))
  (bind (_x_2 _y_2) (`KismetMathLibrary.BreakVector2D` (`self.maxRandomSpawnPosition`)))
  (return (`KismetMathLibrary.MakeVector` (`KismetMathLibrary.RandomFloatInRange` _x _x_2) (`KismetMathLibrary.RandomFloatInRange` _y _y_2) (`self.zPos`))))

(fn `InitializeUserInterface`
  ;[1 1 1] Win/Lose
  (bind _returnvalue (`|CreateWidget` "/Game/Blueprints/UI/WinLoseWidget.WinLoseWidget_C"))
  (`Widget.SetVisibility` _returnvalue "Hidden")
  (`UserWidget.AddToViewport` _returnvalue 0)
  (set `self.winLoseWidget` _returnvalue)
  (bind _returnvalue_2 (`|CreateWidget` "/Game/Blueprints/UI/CountdownGameStart.CountdownGameStart_C"))
  (`Widget.SetVisibility` _returnvalue_2 "Hidden")
  (`UserWidget.AddToViewport` _returnvalue_2 0)
  (bind _output_get (set `self.CountDownUI` _returnvalue_2))
  (`/Game/Blueprints/UI/CountdownGameStart.SetData` _output_get (`self.GamePlayStartText`)))

(fn `MakeGameReady`
  (bind _asgame_instance_ma (cast `/Game/Blueprints/GameInstanceMA` (`GameplayStatics.GetGameInstance`))
    (:`then`
      (bind _output_get (set `self.gameInstanceMA` _asgame_instance_ma))
      (bind _players (`/Game/Blueprints/GameInstanceMA.GetNumberOfPlayers` _output_get))
      (set `self.numPlayers` _players)
      (`self.CreateAllSpawners`)
      (`self.SpawnPlayers`)
      (`self.InitializeUserInterface`))
    (:`CastFailed`
      (`KismetSystemLibrary.PrintString` "Failed casting GameInstanceMA" true true (struct :`R` 1.0 :`G` 0.006772 :`A` 1.0) 10.0))))

(fn `ShowWinLoseUI`
  (params (playerWinName :type String) (round :type Integer))
  (bind _winlosewidget (`self.winLoseWidget`))
  (`KismetSystemLibrary.PrintString` "Show win/lose UI" true true (struct :`G` 0.66 :`B` 1.0 :`A` 1.0) 5.0)
  (`/Game/Blueprints/UI/WinLoseWidget.SetData` _winlosewidget playerWinName round)
  (`Widget.SetVisibility` _winlosewidget "Visible")
  (`/Game/Blueprints/UI/WinLoseWidget.StartAnimation` _winlosewidget))

(fn `SpawnPlayers`
  (for (_array_element _array_index) (`self.Spawners`)
    (`/Game/Blueprints/Spawner.SpawnPlayer` _array_element _array_index (`self.controllerAxis`)))
  (`KismetSystemLibrary.PrintString` "Spawning Players done" true true (struct :`R` 0.413426 :`G` 1.0 :`A` 1.0) 5.0))

(fn `UpdateCountDownUI`
  (params (CountDownTime :type Integer))
  (bind _countdownui (`self.CountDownUI`))
  (bind _countdownui_2 (`self.CountDownUI`))
  (if (!= CountDownTime 0)
    (`/Game/Blueprints/UI/CountdownGameStart.SetCountDownDigit` _countdownui_2 CountDownTime)
    (`/Game/Blueprints/UI/CountdownGameStart.StartAnimation` _countdownui_2)
    (else
      (`/Game/Blueprints/UI/CountdownGameStart.SetCountDownText` _countdownui (`self.GamePlayStartText`))
      (`/Game/Blueprints/UI/CountdownGameStart.StartAnimation` _countdownui))))

(fn `UserConstructionScript`)