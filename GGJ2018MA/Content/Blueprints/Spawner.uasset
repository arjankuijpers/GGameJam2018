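; Spawner actor that creates a local player and places its pawn at the spawner's location.
; SpawnPlayer calls CreatePlayer with pawn spawning, moves the new controller's pawn here, then initializes it with the given index and stores it.
; Debug prints report success or failed casts, and GetPlayerRef exposes the stored Player.
; The event graph is empty, so spawning runs only when SpawnPlayer is called externally.
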(fn `GetPlayerRef`
  (returns (PlayerRef :type "/Game/Blueprints/Player Object Reference"))
  (return (`self.playerRef`)))

(fn `SpawnPlayer`
  (params (index :type Integer))
  (bind _returnvalue (`GameplayStatics.CreatePlayer` -1))
  (bind _asplayer_controller_custom (cast `/Game/Blueprints/PlayerControllerCustom` _returnvalue)
    (:`then`
      (bind _returnvalue_2 (`Controller.K2_GetPawn` _asplayer_controller_custom))
      (`self.K2_SetActorLocation` _returnvalue_2 (`self.K2_GetActorLocation`) false false)
      (bind _asplayer (cast `/Game/Blueprints/Player` _returnvalue_2)
        (:`then`
          (bind _output_get (set `self.playerRef` _asplayer))
          (`/Game/Blueprints/Player.Initialize` _output_get index)
          (`KismetSystemLibrary.PrintString` "Player is spawned" true true (struct :`R` 0.044486 :`G` 0.692708 :`A` 1.0) 5.0))
        (:`CastFailed`
          (`KismetSystemLibrary.PrintString` "Create player failed" true true (struct :`R` 0.692708 :`B` 0.028332 :`A` 1.0) 10.0))))
    (:`CastFailed`
      (`KismetSystemLibrary.PrintString` "Create player failed" true true (struct :`R` 0.692708 :`B` 0.028332 :`A` 1.0) 10.0))))

(fn `UserConstructionScript`)