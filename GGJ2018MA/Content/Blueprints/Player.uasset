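; Player actor that moves itself forward each tick while activated, at a speed scaled by a buff multiplier with a minimum floor.
; Overlapping Obstacle actors add their speed multiplier and switch color, then undo both on exit.
; Exposed functions toggle movement, set speed and yaw-only heading, apply turn input, and assign the player index with its matching body material.
; Movement sets location directly without sweep; an older swept version remains unused.
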(event `self.ReceiveTick`
  (params (DeltaSeconds :type "Float (single-precision)"))
  (if (`self.activated`)
    ;[1 1 1] New Implementation (uses Player Controller)
    (`self.K2_SetActorLocation` (+ (* (`KismetMathLibrary.GetForwardVector` (`self.K2_GetActorRotation`)) (* DeltaSeconds (* (`self.speed`) (`KismetMathLibrary.FMax` (`self.speedBuffMultiplier`) (`self.minimalSpeedBuffMultiplier`))))) (`self.K2_GetActorLocation`)))))

(event `self.ReceiveActorBeginOverlap`
  (params (OtherActor :type "Actor Object Reference"))
  (`KismetSystemLibrary.PrintString` "Player start overlap with obstacle")
  (if (`KismetMathLibrary.ClassIsChildOf` (`GameplayStatics.GetObjectClass` OtherActor) "/Game/Blueprints/obstacles/Obstacle.Obstacle_C")
    (bind _asobstacle (cast `/Game/Blueprints/obstacles/Obstacle` OtherActor)
      (:`then`
        (bind _output_get (set `self.speedBuffMultiplier` (+ (`self.speedBuffMultiplier`) (`/Game/Blueprints/obstacles/Obstacle.speedMultiplier` _asobstacle))))
        (`KismetSystemLibrary.PrintString` (`KismetStringLibrary.Concat_StrStr` "Player Speed: " (`KismetStringLibrary.Conv_DoubleToString` _output_get)) true true (struct :`G` 0.66 :`B` 1.0 :`A` 1.0) 5.0)
        (`/Game/Blueprints/obstacles/Obstacle.SetColorPlayerActive` _asobstacle))
      (:`CastFailed`
        (`KismetSystemLibrary.PrintString` "Obstacle cast failed." true true (struct :`R` 1.0 :`B` 0.023006 :`A` 1.0) 5.0)))))

(event `self.ReceiveActorEndOverlap`
  (params (OtherActor :type "Actor Object Reference"))
  (`KismetSystemLibrary.PrintString` "Player end overlap with obstacle")
  (if (`KismetMathLibrary.ClassIsChildOf` (`GameplayStatics.GetObjectClass` OtherActor) "/Game/Blueprints/obstacles/Obstacle.Obstacle_C")
    (bind _asobstacle (cast `/Game/Blueprints/obstacles/Obstacle` OtherActor)
      (:`then`
        (bind _output_get (set `self.speedBuffMultiplier` (- (`self.speedBuffMultiplier`) (`/Game/Blueprints/obstacles/Obstacle.speedMultiplier` _asobstacle))))
        (`KismetSystemLibrary.PrintString` (`KismetStringLibrary.Concat_StrStr` "Player Speed: " (`KismetStringLibrary.Conv_DoubleToString` _output_get)) true true (struct :`G` 0.66 :`B` 1.0 :`A` 1.0) 5.0)
        (`/Game/Blueprints/obstacles/Obstacle.SetColorNoPlayerActive` _asobstacle))
      (:`CastFailed`
        (`KismetSystemLibrary.PrintString` "Obstacle cast failed." true true (struct :`R` 1.0 :`B` 0.023006 :`A` 1.0) 5.0)))))

(fn `ActivateMovement`
  (set `self.activated` true))

(fn `AddDirectionRotation`
  (params (rotation :type "Rotator Structure"))
  (bind (_rotation_roll _rotation_pitch _rotation_yaw) (`KismetMathLibrary.BreakRotator` (`self.rotation`)))
  (bind _output_get (set `self.rotation` (`KismetMathLibrary.MakeRotator` 0.0 0.0 (+ _rotation_yaw (* rotation_Yaw (`self.rotationSpeed`))))))
  (`self.K2_SetActorRotation` _output_get))

(fn `DeactivateMovement`
  (set `self.activated` false))

(fn `GetDirectionRotation`
  (returns (currentRotation :type "Rotator Structure"))
  (return (`self.rotation`)))

(fn `GetPlayerIndex`
  (returns (GetPlayerIndex :type Integer))
  (return (`self.index`)))

(fn `Initialize`
  (params (playerIndex :type Integer))
  (set `self.index` playerIndex)
  (`PrimitiveComponent.SetMaterial` (`self.playerBody`) 0 (`|GetArrayItem` (`self.PlayerMaterialList`) playerIndex))
  (`KismetSystemLibrary.PrintString` "Player material set" true true (struct :`R` 0.318126 :`G` 0.787349 :`B` 1.0 :`A` 1.0) 5.0))

(fn `SetMovementData`
  (params (rotator :type "Rotator Structure") (speed :type "Float (double-precision)") (rotationSpeed :type "Float (double-precision)"))
  (set `self.speed` speed)
  (set `self.rotationSpeed` rotationSpeed)
  (bind _output_get (set `self.rotation` (`KismetMathLibrary.MakeRotator` 0.0 0.0 (.yaw rotator))))
  (`self.K2_SetActorRotation` _output_get))

(fn `UserConstructionScript`)